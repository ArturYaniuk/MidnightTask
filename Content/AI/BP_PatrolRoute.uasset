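; BP_PatrolRoute defines a spline-based patrol path, stored under AI, that tracks a current waypoint along its points.
; IncrementControlRoute steps PatrolIndex by Direction and flips Direction at the first and last spline points, giving a back-and-forth ping-pong order.
; GetSplinePointAsWorldPos returns the world location of the current point.
; GetPatrolRoute and SetMovementSpeed are empty stubs here, the latter returning zero.
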(event `IncrementControlRoute`
  (bind _output_get (set `self.PatrolIndex` (+ (`self.PatrolIndex`) (`self.Direction`))))
  (if (== _output_get (- (`SplineComponent.GetNumberOfSplinePoints` (`self.PatrolRout`)) 1))
    (set `self.Direction` -1)
    (elif (== (`self.PatrolIndex`) 0)
      (set `self.Direction` 1))))

(fn `Get Spline Point As World Pos`
  (returns (ReturnValue :type "Vector Structure"))
  (return (`SplineComponent.GetLocationAtSplinePoint` (`self.PatrolRout`) (`self.PatrolIndex`) "World")))

(fn `GetPatrolRoute`
  (returns (PatrolRoute :type "/Game/AI/BP_PatrolRoute Object Reference"))
  (return null))

(fn `SetMovementSpeed`
  (params (Speed :type "/Game/AI/Enums/E_MovementSpeed Enum" :default "NewEnumerator0"))
  (returns (SpeedValue :type "Float (double-precision)"))
  (return 0.0))

(fn `UserConstructionScript`)