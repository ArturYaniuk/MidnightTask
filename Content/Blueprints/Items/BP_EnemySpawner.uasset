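; Enemy spawner actor that periodically creates AI enemies around its own location.
; On BeginPlay it caches the BP_GameMod game mode and starts a looping timer.
; Each tick of the timer spawns a BP_Enemy running BT_Enemy_Base at a random reachable nearby point, unless the game mode's alive count exceeds its maximum.
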(event `SpawnEnemy`
  (if (not (> (`/Game/BP_GameMod.EnemyAlive` (stale `self.ReceiveBeginPlay` _asbp_game_mod)) (`/Game/BP_GameMod.MaxEnemy` (stale `self.ReceiveBeginPlay` _asbp_game_mod))))
    (`AIBlueprintHelperLibrary.SpawnAIFromClass` "/Game/Blueprints/Characters/BP_Enemy.BP_Enemy_C" "/Game/AI/BT_Enemy_Base.BT_Enemy_Base" (`NavigationSystemV1.K2_GetRandomReachablePointInRadius` (`self.K2_GetActorLocation`) 100.0 null null) (struct) false null)))

(event `self.ReceiveBeginPlay`
  (bind _asbp_game_mod (cast `/Game/BP_GameMod` (`GameplayStatics.GetGameMode`)))
  (`KismetSystemLibrary.K2_SetTimerDelegate` (delegate `SpawnEnemy`) 2.0 true))

(fn `UserConstructionScript`)